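; Assault rifle weapon Blueprint that identifies itself as an AK rifle starting in the Dropped state.
; BeginPlay runs the parent logic, then fills WeaponData with the name, type and state.
; Tick prints on-screen debug text every frame showing whether the Collision and WeaponBody components are simulating physics.
; The construction script only calls its parent.
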(event `self.ReceiveBeginPlay`
  (`parent.ReceiveBeginPlay`)
  (set `self.WeaponData` (make `WeaponData` "AK" "EHWT_Rifle")))

(event `self.ReceiveTick`
  (params (DeltaSeconds :type "Float (single-precision)"))
  (`KismetSystemLibrary.PrintString` (`KismetStringLibrary.Concat_StrStr` "Collision Physics:" (`KismetStringLibrary.Conv_BoolToString` (`SceneComponent.IsSimulatingPhysics` (`self.Collision`) "None"))) true true (struct :`G` 0.66 :`B` 1.0 :`A` 1.0) 0.0)
  (`KismetSystemLibrary.PrintString` (`KismetStringLibrary.Concat_StrStr` "Weapon Physics:" (`KismetStringLibrary.Conv_BoolToString` (`SceneComponent.IsSimulatingPhysics` (`self.WeaponBody`) "None"))) true true (struct :`G` 0.66 :`B` 1.0 :`A` 1.0) 0.0))

(fn `UserConstructionScript`
  (`parent.UserConstructionScript`))