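; Pistol weapon Blueprint, a child of a weapon base, that fires physical bullets toward where the player's camera is aimed.
; On fire it calls the parent, then line-traces from the camera on Visibility with persistent debug drawing, ignoring itself and the player pawn.
; It spawns a Bullet_bp at the Barrel socket with velocity toward the impact point, without checking for a hit.
; The construction script sets weapon data and hand transform.
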(event `self.ReceiveBeginPlay`
  (set `self.Ignores` (`|MakeArray` self (`GameplayStatics.GetPlayerPawn` 0) :!type "Actor Object Reference")))

(event `self.FireWeapon`
  (params (PlayerCamera :type "CameraComponent Object Reference"))
  (bind _returnvalue (`SceneComponent.K2_GetComponentLocation` PlayerCamera))
  (bind _returnvalue_2 (`SceneComponent.GetSocketLocation` (`self.WeaponBody`) "Barrel"))
  (`parent.FireWeapon` PlayerCamera)
  (bind _outhit (`KismetSystemLibrary.LineTraceSingle` _returnvalue (+ _returnvalue (* (`SceneComponent.GetForwardVector` PlayerCamera) 10000.0)) "TraceTypeQuery1" false (`self.Ignores`) "Persistent" true (struct :`R` 1.0 :`A` 1.0) (struct :`G` 1.0 :`A` 1.0) 0.0))
  (bind _output_get (set `self.HitPoint` _outhit))
  (`|SpawnActorFromClass` "/Game/Blueprints/Items/bullet_bp.bullet_bp_C" (`KismetMathLibrary.MakeTransform` _returnvalue_2) "AlwaysSpawn" "OverrideRootScale" null (* (`KismetMathLibrary.Normal` (- (`.ImpactPoint` (`GameplayStatics.BreakHitResult` _output_get)) _returnvalue_2)) 10000.0) null))

(fn `UserConstructionScript`
  (set `self.WeaponData` (make `WeaponData` "Pistol" "EHWT_Pistol"))
  (set `self.HandTransform` (`KismetMathLibrary.MakeTransform` (0.0 0.0 0.0) (struct))))