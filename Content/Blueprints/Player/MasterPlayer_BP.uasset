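; MasterPlayer_BP is a player Blueprint that handles movement, camera look and an interact action.
; Axis inputs drive movement along the controller rotation's forward and right vectors, plus yaw and pitch, while pressing Interact calls an Interact function.
; An UpdateAttachment event snaps the HandedWeapon component to the mesh's ik_hand_gun socket.
; Tick prints the handed weapon's name on screen as debug output.
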(event `InputAxis|MoveForward`
  (params (AxisValue :type "Float (single-precision)"))
  (bind _output_get (set `self.MoveForward` AxisValue))
  (`self.AddMovementInput` (`self.ControllerRotation`) _output_get))

(event `InputAxis|Turn`
  (params (AxisValue :type "Float (single-precision)"))
  (bind _output_get (set `self.TurnValue` AxisValue))
  (`self.AddControllerYawInput` _output_get))

(event `InputAxis|LookUp`
  (params (AxisValue :type "Float (single-precision)"))
  (bind _output_get (set `self.LookValue` AxisValue))
  (`self.AddControllerPitchInput` _output_get))

(event `InputAxis|MoveRight`
  (params (AxisValue :type "Float (single-precision)"))
  (bind _output_get (set `self.MoveRight` AxisValue))
  (`self.AddMovementInput` (`.RightVector` (`self.ControllerRotation`)) _output_get))

(event `InputAction|Interact`
  (params (Key :type "Key Structure"))
  (:`Pressed`
    (`self.Interact`)))

(event `self.UpdateAttachment`
  (`self.K2_AttachToComponent` (`self.HandedWeapon`) (`self.Mesh`) "ik_hand_gun" "SnapToTarget" "SnapToTarget" "SnapToTarget" true))

(event `self.ReceiveTick`
  (params (DeltaSeconds :type "Float (single-precision)"))
  (`KismetSystemLibrary.PrintString` (`KismetStringLibrary.Concat_StrStr` "Handed Weapon: " (`KismetSystemLibrary.GetDisplayName` (`self.HandedWeapon`))) true true (struct :`G` 0.66 :`B` 1.0 :`A` 1.0) 0.0))

(fn `UserConstructionScript`)